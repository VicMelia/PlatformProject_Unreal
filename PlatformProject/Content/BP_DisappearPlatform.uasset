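; BP_DisappearPlatform is a platform that periodically disappears and reappears.
; On BeginPlay it starts a looping timer using the Timer variable as its interval.
; Each tick of that timer toggles the Cube's visibility, then sets its collision to query-and-physics when visible or none when hidden.
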(event `self.ReceiveBeginPlay`
  (`KismetSystemLibrary.K2_SetTimerDelegate` (delegate `AlternateBlock`) (`self.Timer`) true))

(event `AlternateBlock`
  (bind _cube (`self.Cube`))
  (bind _cube_2 (`self.Cube`))
  (`SceneComponent.SetVisibility` _cube_2 (not (`SceneComponent.IsVisible` _cube_2)) false)
  (if (`SceneComponent.IsVisible` _cube)
    (`PrimitiveComponent.SetCollisionEnabled` _cube "QueryAndPhysics")
    (else
      (`PrimitiveComponent.SetCollisionEnabled` _cube "NoCollision"))))

(fn `UserConstructionScript`)